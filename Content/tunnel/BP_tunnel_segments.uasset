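; Tunnel segment Blueprint that builds a chain of deformed mesh pieces along an editable spline.
; The construction script divides the spline length by SectionLength and adds a Y-forward spline mesh component for each index, including the truncated final one.
; Each piece takes local positions and tangents from the spline at its two ends, with tangent size clamped to SectionLength.
; The event graph holds no runtime logic.
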(fn `UserConstructionScript`
  (bind _section_length (`self.section length`))
  (bind _spline (`self.Spline`))
  (bind _spline_2 (`self.Spline`))
  (for _index (range (+ (`KismetMathLibrary.FTrunc` (/ (`SplineComponent.GetSplineLength` (`self.Spline`)) (`self.section length`))) 1))
    (bind _returnvalue (`AddComponent|NODE_AddSplineMeshComponent-0`))
    (`SplineMeshComponent.SetForwardAxis` _returnvalue "Y" true)
    (bind _returnvalue_2 (* _index _section_length))
    (bind _returnvalue_3 (* (+ _index 1) _section_length))
    (`SplineMeshComponent.SetStartAndEnd` _returnvalue (`SplineComponent.GetLocationAtDistanceAlongSpline` _spline_2 _returnvalue_2 "Local") (`KismetMathLibrary.ClampVectorSize` (`SplineComponent.GetTangentAtDistanceAlongSpline` _spline_2 _returnvalue_2 "Local") 0.0 (`self.section length`)) (`SplineComponent.GetLocationAtDistanceAlongSpline` _spline _returnvalue_3 "Local") (`KismetMathLibrary.ClampVectorSize` (`SplineComponent.GetTangentAtDistanceAlongSpline` _spline _returnvalue_3 "Local") 0.0 (`self.section length`)) true)))